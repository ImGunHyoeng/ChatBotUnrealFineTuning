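; BP_ChatBot is an actor that runs an OpenAI-backed chat bot and shows its replies in the WB_Chat widget.
; ChatBotRequest sets a hardcoded API key, caches the widget, appends the input to a running ChatLog and sends the whole log to a fine-tuned GPT-3.5 Turbo model.
; Successful replies join the log and go to the widget's Result; failures only print the error.
; An older Davinci completion call is left unconnected.
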(event Custom|ChatBotRequest
  (params (input :type Chat%20Log%20Structure))
  (bind _chatlog (Variables|Default|GetChatLog))
  ;[1 1 1] API키 설정
  (Development|PrintString (.content (Utilities|Struct|BreakChatLog input)))
  (Class|OpenAIUtils|SetOpenAIApiKey "sk-None-G34QDfqYK2fKFMPuCGBdT3BlbkFJf6Df8nmo7D68YaDGBJzl")
  ;[1 1 1] null 체크
  (if (== (Variables|Default|GetAs%20WB%20Chat) 0)
    ;[1 1 1] 위젯 설정
    (bind _foundwidgets (Widget|GetAllWidgetsOfClass "/Game/Chat/HUD/WB_Chat.WB_Chat_C" true))
    (Variables|Default|SetAs%20WB%20Chat (Utilities|Array|Get(acopy) _foundwidgets)))
  ;[1 1 1] 지피티 4용 버전
  (Utilities|Array|Add _chatlog input)
  (bind (_message _errormessage _success) (|OpenAICallChat (Utilities|Struct|MakeChatSettings "GPT_3_5_TURBO_FineTunning_V2" _chatlog 0.2 400))
    (:Finished
      (if _success
        (Utilities|Array|Add (Variables|Default|GetChatLog) (.message (Utilities|Struct|BreakChatCompletion _message)))
        (Development|PrintString (.content (Utilities|Struct|BreakChatLog (.message (Utilities|Struct|BreakChatCompletion _message)))) true true "(R=0.000000,G=0.660000,B=1.000000,A=1.000000)" 1e+01)
        (Default|Result (Variables|Default|GetAs%20WB%20Chat) (Utilities|Text|ToText(String) (.content (Utilities|Struct|BreakChatLog (.message (Utilities|Struct|BreakChatCompletion _message))))))
        (else
          (Development|PrintString _errormessage))))))

(event EventBeginPlay)

(event Collision|EventActorBeginOverlap
  (params (OtherActor :type Actor%20Object%20Reference)))

(event EventTick
  (params (DeltaSeconds :type Float%20%28single-precision%29)))

(fn ConstructionScript)